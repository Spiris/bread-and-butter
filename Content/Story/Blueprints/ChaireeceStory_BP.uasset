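; Story component for Chairman Chaireece that plays a linear, comedic three-speaker conversation with Chairles and Chairry, ending in lorem ipsum filler.
; On BeginPlay it sets character names and caches "Story"-tagged anchor components for the owner and the referenced Bob and Frank actors, with the owner's setup nested inside both validity checks.
; The story graph chains one-way text nodes, switches speakers through validity-checked helper functions, and calls Cancel at the end.
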(event `self.ReceiveBeginPlay`
  (bind _returnvalue (`self.GetOwner`))
  (`parent.ReceiveBeginPlay`)
  (bind _bobthechairsactor (`self.BobTheChairsActor`)
    (:`then`
      (set `CharacterComponent.CharacterName` (`KismetTextLibrary.Conv_TextToString` (`self.BobsOtherName`)) (`Actor.GetComponentByClass` _bobthechairsactor "/Script/BNB.CharacterComponent"))
      (set `self.BobsComponent` (`|GetArrayItem` (`Actor.GetComponentsByTag` _bobthechairsactor "/Script/Engine.SceneComponent" "Story")))
      (bind _franktheactor (`self.FrankTheActor`)
        (:`then`
          (set `CharacterComponent.CharacterName` (`KismetTextLibrary.Conv_TextToString` (`self.FraksOtherName`)) (`Actor.GetComponentByClass` _franktheactor "/Script/BNB.CharacterComponent"))
          (set `self.FranksComponent` (`|GetArrayItem` (`Actor.GetComponentsByTag` _franktheactor "/Script/Engine.SceneComponent" "Story")))
          (set `CharacterComponent.CharacterName` (`KismetTextLibrary.Conv_TextToString` (`self.ChaireeceName`)) (`Actor.GetComponentByClass` _returnvalue "/Script/BNB.CharacterComponent"))
          (set `self.MyComponent` (`|GetArrayItem` (`Actor.GetComponentsByTag` _returnvalue "/Script/Engine.SceneComponent" "Story"))))
        (:`else`)))
    (:`else`)))

(event `self.OnStoryBeginGraph_BP`
  (`self.ChangeSpeakerToSelfAKAChaireece`)
  (`|FoldingSkyStoryOneWayText` "Good day to you sir, I am Chairman Chaireece. It is a pleasure to meet you."
    (:`OnWayOne`
      (`self.ChangeSpeakerToBobAKAChairles`)
      (`|FoldingSkyStoryOneWayText` "Good day to you sir, I am second chair Chairles, would you like to meet mour collaborator Chairry?"
        (:`OnWayOne`
          (`self.ChangeSpeakerToFrankAKAChairry`)
          (`|FoldingSkyStoryOneWayText` "Too bad I don't want to talk to you."
            (:`OnWayOne`
              (`self.ChangeSpeakerToSelfAKAChaireece`)
              (`|FoldingSkyStoryOneWayText` "Really missed out on that one, prepare now for your lorem ipsum punishment."
                (:`OnWayOne`
                  (`|FoldingSkyStoryOneWayText` ". . ."
                    (:`OnWayOne`
                      (`|FoldingSkyStoryOneWayText` "Lorem"
                        (:`OnWayOne`
                          (`|FoldingSkyStoryOneWayText` "Ipsum"
                            (:`OnWayOne`
                              (`|FoldingSkyStoryOneWayText` "Dolor"
                                (:`OnWayOne`
                                  (`|FoldingSkyStoryOneWayText` "Sed ut perspiciatis unde omnis iste natus error sit voluptatem accusantium doloremque laudantium, totam rem aperiam, eaque ipsa quae ab illo inventore veritatis et quasi architecto beatae vitae dicta sunt explicabo."
                                    (:`OnWayOne`
                                      (`|FoldingSkyStoryOneWayText` "Nemo enim ipsam voluptatem quia voluptas sit aspernatur aut odit aut fugit, sed quia consequuntur magni dolores eos qui ratione voluptatem sequi nesciunt."
                                        (:`OnWayOne`
                                          (`|FoldingSkyStoryOneWayText` "Neque porro quisquam est, qui dolorem ipsum quia dolor sit amet, consectetur, adipisci velit, sed quia non numquam eius modi tempora incidunt ut labore et dolore magnam aliquam quaerat voluptatem. Ut enim ad minima veniam, quis nostrum exercitationem ullam corporis suscipit laboriosam, nisi ut aliquid ex ea commodi consequatur?"
                                            (:`OnWayOne`
                                              (`|FoldingSkyStoryOneWayText` "Quis autem vel eum iure reprehenderit qui in ea voluptate velit esse quam nihil molestiae consequatur, vel illum qui dolorem eum fugiat quo voluptas nulla pariatur?"
                                                (:`OnWayOne`
                                                  (`self.Cancel`))))))))))))))))))))))))))

(fn `ChangeSpeakerToBobAKAChairles`
  (bind _bobscomponent (`self.BobsComponent`)
    (:`then`
      (`self.ChangeSpeaker` _bobscomponent (`self.BobsOtherName`)))
    (:`else`)))

(fn `ChangeSpeakerToFrankAKAChairry`
  (bind _frankscomponent (`self.FranksComponent`)
    (:`then`
      (`self.ChangeSpeaker` _frankscomponent (`self.FraksOtherName`)))
    (:`else`)))

(fn `ChangeSpeakerToSelfAKAChaireece`
  (bind _mycomponent (`self.MyComponent`)
    (:`then`
      (`self.ChangeSpeaker` _mycomponent (`self.ChaireeceName`)))
    (:`else`)))