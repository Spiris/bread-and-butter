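; StatusReportText_BP is a pop-up status text actor that launches upward, arcs back down and turns toward the camera.
; BeginPlay seeds a velocity with a strong upward kick and slight random positive X/Y drift.
; Tick applies hand-rolled gravity, overwrites the root's physics linear velocity, then calls FaceCamera.
; An inline look-at rotation toward the player camera is left disconnected and never runs.
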(event `self.ReceiveBeginPlay`
  (bind _returnvalue (* (`KismetMathLibrary.RandomFloat`) 100.0))
  (set `self.Velocity` (`KismetMathLibrary.MakeVector` _returnvalue _returnvalue 900.0)))

(event `self.ReceiveTick`
  (params (DeltaSeconds :type "Float (single-precision)"))
  (bind (_velocity_x _velocity_y _velocity_z) (`KismetMathLibrary.BreakVector` (`self.Velocity`)))
  (bind _output_get (set `self.Velocity` (`KismetMathLibrary.MakeVector` _velocity_x _velocity_y (- _velocity_z (* DeltaSeconds 2300.0)))))
  (`PrimitiveComponent.SetPhysicsLinearVelocity` (`self.Root`) _output_get false "None")
  (`CoreFunctionLibrary.FaceCamera` self))

(fn `UserConstructionScript`)