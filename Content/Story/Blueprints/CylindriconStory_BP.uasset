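; Branching dialogue story for Cylindricon, a comedic NPC who gates conversation behind the player proving worthy.
; StoryGraph checks IsWorthy on story begin, offering either an animal-noise menu or a dismissive challenge that can lead to an egg-preference quiz.
; Answering Benedict sets IsWorthy, changes the speaker to reveal the name and portrait, then jumps into the worthy menu.
; Other endings route through SayGoodbye, which says farewell and cancels the story.
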(event `self.OnStoryBeginGraph_BP`
  (if (`self.bIsWorthy`)
    (`|FoldingSkyStoryTwoWayText` "Hey wanna know something?"
      (:`OnWayOne`
        (`|FoldingSkyStoryWithChoicesText` "What can I do for you?" "moo" "baa" "ree" "caw" :!label _label
          (:`OnChoice1`
            (`|FoldingSkyStoryOneWayText` "okay. MOOOOOOoooOoOOoOoooooo"
              (:`OnWayOne`
                _)))
          (:`OnChoice2`
            (`|FoldingSkyStoryOneWayText` "okay. OH MAAAAAAAAAAAa"
              (:`OnWayOne`
                _)))
          (:`OnChoice3`
            (`|FoldingSkyStoryOneWayText` "BASHIIIIII"
              (:`OnWayOne`
                _)))
          (:`OnChoice4`
            (`|FoldingSkyStoryOneWayText` "BUCAWK"
              (:`OnWayOne`
                _))))
        (`self.SayGoodbye`))
      (:`OnWayTwo`
        (`|FoldingSkyStoryOneWayText` "WELL FINE"
          (:`OnWayOne`
            (`self.SayGoodbye` :!label _label_2)))))
    (else
      (`|FoldingSkyStoryTwoWayText` "You are not worthy to speak to me. Do you think you are special or something?"
        (:`OnWayOne`
          (`|FoldingSkyStoryOneWayText` "WELL YOU ARE NOT"
            (:`OnWayOne`
              (goto _label_2))))
        (:`OnWayTwo`
          (`|FoldingSkyStoryWithChoicesText` "Well, maybe there is hope for you yet. \n \nHow do you like your eggs?" "Scrambled" "Over easy" "Over medium" "Over hard" "Benedict" "Raw"
            (:`OnChoice1`
              (`|FoldingSkyStoryOneWayText` "Yikes"
                (:`OnWayOne`
                  _)))
            (:`OnChoice2`
              (`|FoldingSkyStoryOneWayText` "Eff"
                (:`OnWayOne`
                  _)))
            (:`OnChoice3`
              (`|FoldingSkyStoryOneWayText` "Hmmm... interesting choice."
                (:`OnWayOne`
                  _)))
            (:`OnChoice4`
              (`|FoldingSkyStoryOneWayText` "OOOF"
                (:`OnWayOne`
                  _)))
            (:`OnChoice5`
              (`self.ChangeSpeaker` (`Actor.RootComponent` (`self.GetOwner`)) "Cylyndricon" "/Engine/EditorResources/Ai_Spawnpoint.Ai_Spawnpoint")
              (set `self.bIsWorthy` true)
              (`|FoldingSkyStoryOneWayText` "I see... YOU ARE THE CHOSEN ONE THE PROPHECIES FORETOLD! \nYou may call me Cylindricon, hero."
                (:`OnWayOne`
                  (goto _label))))
            (:`OnChoice6`
              (`|FoldingSkyStoryOneWayText` "Holy cow! Holy cow! Holy cow!"
                (:`OnWayOne`
                  _))))
          (`self.SayGoodbye`))))))

(event `SayGoodbye`
  (`|FoldingSkyStoryOneWayText` "Farewell!"
    (:`OnWayOne`
      (`self.Cancel`))))