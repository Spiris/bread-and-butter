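; Narrator intro story graph: a comedic voiced questionnaire about romantic preferences that ends with the player married to their spacebar.
; After a greeting, it chains six six-choice questions where only the last, spacebar-themed answer advances and updates Stage.
; While IsHandlingErrors is set, any other accepted choice plays a random ErrorDialogues line, then re-asks the current Stage's question.
; The final correct answer clears that flag, shows the closing text and cancels the story.
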(event `HandleIncorrectChoice`
  (bind _errordialogues (`self.ErrorDialogues`))
  (`|FoldingSkyStoryOneWayDialogue` (`|GetArrayItem` _errordialogues (`KismetMathLibrary.RandomIntegerInRange` 0 (- (`KismetArrayLibrary.Array_Length` _errordialogues) 1)))
    (:`OnWayOne`
      (switch `int` (`self.Stage`)
        (:`0`
          (`|FoldingSkyStoryWithChoicesDialogue` "/Game/Story/DialogueWaves/NarratorIntroGenderPref_DW.NarratorIntroGenderPref_DW" "I like men!  men! men! men! Manly men!" "I like women! Only women!" "I consider myself a bit of an explorer, actually." "Androgynous only please." "I prefer people with multitools." "I really like my spacebar... it is a good spacebar." :!label _label
            (:`OnChoice6`
              (set `self.Stage` 1)
              (`|FoldingSkyStoryWithChoicesDialogue` "/Game/Story/DialogueWaves/NarratorIntroNumberPref_DW.NarratorIntroNumberPref_DW" "Just one." "Ive always dreamed of two at once..." "At least 3, maybe more." "Negative 1, like an antimatter inverted person." "None." "All I need is my spacebar." :!label _label_2
                (:`OnChoice6`
                  (set `self.Stage` 2)
                  (`|FoldingSkyStoryWithChoicesDialogue` "/Game/Story/DialogueWaves/NarratorIntroFetishPref_DW.NarratorIntroFetishPref_DW" "I like to choke while it happens." "Frilly clothes. Maybe slime?" "Shiny clothes. Maybe robots." "Washboard abs and THICCC thighs." "I like em BIG BIG BIG." "Long, slender, shaped like a spacebar... is this normal?" :!label _label_3
                    (:`OnChoice6`
                      (set `self.Stage` 3)
                      (`|FoldingSkyStoryWithChoicesDialogue` "/Game/Story/DialogueWaves/NarratorIntroFetishPref_DW_2.NarratorIntroFetishPref_DW_2" "Never, I was joking. It was a joke." "Sometimes." "Often." "Rarely. Really just once." "I don't know." "How many stars are in the sky? How often do they burn? My spacebar calls to me, even now." :!label _label_4
                        (:`OnChoice6`
                          (set `self.Stage` 4)
                          (`|FoldingSkyStoryWithChoicesDialogue` "/Game/Story/DialogueWaves/NarratorIntroColorPref_DW.NarratorIntroColorPref_DW" "White as the Aryan Sun." "Like my coffee, black." "Like my coffee, mocha." "Like my coffee, pumpkin spice!" "All the colors of the rainbow!" "What color does my spacebar like? do you think it likes me?" :!label _label_5
                            (:`OnChoice6`
                              (set `self.Stage` 5))))))))))))
        (:`1`
          (goto _label_2))
        (:`2`
          (goto _label_3))
        (:`3`
          (goto _label_4))
        (:`4`
          (goto _label_5))
        (:`5`
          _))
      (`|FoldingSkyStoryWithChoicesDialogue` "/Game/Story/DialogueWaves/NarratorIntroAgePref_DW.NarratorIntroAgePref_DW" "I... I am going to jail." "Over the age of consent!" "Thousand year old dragons only." "Define.... age?" "Yeeeeeeeeeee" "My spacebar is as timeless as the cosmos and as beautiful as the fabric of eternity."
        (:`OnChoice6`
          (set `self.bIsHandlingErrors` false)
          (`|FoldingSkyStoryOneWayText` "Well done, you are now married to your spacebar."
            (:`OnWayOne`
              (`self.Cancel`))))))))

(event `self.OnStoryBeginGraph_BP`
  (`|FoldingSkyStoryOneWayDialogue` "/Game/Story/DialogueWaves/NarratorIntroGreeting_DW.NarratorIntroGreeting_DW"
    (:`OnWayOne`
      (set `self.Stage` 0)
      (goto _label))))

(event `self.OnStoryChoiceAccepted_BP`
  (params (Choice :type "Integer (by ref)") (ChoiceText :type "Text (by ref)"))
  (if (`self.bIsHandlingErrors`)
    (if (!= Choice 5)
      (`self.HandleIncorrectChoice`))))